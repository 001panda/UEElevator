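; Elevator actor whose two doors the player opens and closes manually with the F key.
; A box overlap with BP_Player flags the player as in front, and toggling requires that flag and the elevator not running.
; A FlipFlop plays or reverses a timeline that slides the doors in opposite directions along their forward vectors via CalculateDoor, from relative positions cached at BeginPlay.
; No elevator travel logic is present.
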(event `self.ReceiveBeginPlay`
  (`self.SoveDoorLovecationPreMove`))

(event `SoveDoorLovecationPreMove`
  ;[1 1 1] 保存门移动的位置
  (set `self.Door1LocationPreMove` (`SceneComponent.RelativeLocation` (`self.door1`)))
  (set `self.Door2Location` (`SceneComponent.RelativeLocation` (`self.door2`))))

(event `Open or Close Door`
  (bind _door1 (`self.door1`))
  (bind _door2 (`self.door2`))
  ;[1 1 1] 实现电梯的开关门
  (if (and (`self.Is Elevator Forward`) (not (`self.Is Elevator Running`)))
    (`/Engine/EditorBlueprintResources/StandardMacros.FlipFlop`
      (:`A`
        (bind (_direction _alpha) (`Timeline|TL_OnOffDorr` :`NewTime` 3.0 :!label _label)
          (:`Update`
            (`|ExecutionSequence`
              (:`then_0`
                (`SceneComponent.K2_SetRelativeLocation` _door1 (`self.CalculateDoor` (`self.Door1LocationPreMove`) _door1 _alpha -1.0) false false))
              (:`then_1`
                (`SceneComponent.K2_SetRelativeLocation` _door2 (`self.CalculateDoor` (`self.Door2Location`) _door2 _alpha 1.0) false false))))))
      (:`B`
        (goto _label :!via `Reverse`)))))

(event `Key|F`
  (params (Key :type "Key Structure"))
  ;[1 1 1] 实现电梯的开关门
  (:`Pressed`
    (`self.Open or Close Door`)))

(event `self.Box.OnComponentBeginOverlap`
  (params (OverlappedComponent :type "PrimitiveComponent Object Reference") (OtherActor :type "Actor Object Reference") (OtherComp :type "PrimitiveComponent Object Reference") (OtherBodyIndex :type Integer) (bFromSweep :type Boolean) (SweepResult :type "HitResult Structure (by ref)"))
  ;[1 1 1] 角色是否移动到电梯前，才能手动打开电梯
  (cast `/Game/TEST_DIANTI/Blueprints/Player/BP_Player` OtherActor)
  (set `self.Is Elevator Forward` true))

(event `self.Box.OnComponentEndOverlap`
  (params (OverlappedComponent :type "PrimitiveComponent Object Reference") (OtherActor :type "Actor Object Reference") (OtherComp :type "PrimitiveComponent Object Reference") (OtherBodyIndex :type Integer))
  ;[1 1 1] 角色是否移动到电梯前，才能手动打开电梯
  (cast `/Game/TEST_DIANTI/Blueprints/Player/BP_Player` OtherActor)
  (set `self.Is Elevator Forward` false))

(fn `CalculateDoor`
  (params (`init Location` :type "Vector Structure") (Door :type "SceneComponent Object Reference") (Alpha :type "Float (double-precision)") (`Left or Right` :type "Float (double-precision)"))
  (returns (CurrentLocation :type "Vector Structure"))
  ;[1 1 1] 函数电梯开关门
  (return (+ `init Location` (* (`SceneComponent.GetForwardVector` Door) (* (`KismetMathLibrary.Lerp` 0.0 200.0 Alpha) `Left or Right`)))))

(fn `UserConstructionScript`)
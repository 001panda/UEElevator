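; BP_Player is the player character Blueprint, handling basic movement, camera look and jumping from input bindings.
; Forward and right axes add movement along directions built from only the control rotation's yaw, keeping movement horizontal regardless of view pitch.
; Pitch and yaw axes feed controller rotation, and the jump action starts Jump on press and StopJumping on release.
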(event `InputAxis|MovementForward`
  (params (AxisValue :type "Float (single-precision)"))
  (bind (_returnvalue_roll _returnvalue_pitch _returnvalue_yaw) (`KismetMathLibrary.BreakRotator` (`self.GetControlRotation`)))
  ;[1 1 1] WASD移动
  (`self.AddMovementInput` (`KismetMathLibrary.GetForwardVector` (`KismetMathLibrary.MakeRotator` 0.0 0.0 _returnvalue_yaw)) AxisValue))

(event `InputAxis|ViewTurnPich`
  (params (AxisValue :type "Float (single-precision)"))
  ;[1 1 1] 视图
  (`self.AddControllerPitchInput` AxisValue))

(event `InputAxis|ViewTurnYaw`
  (params (AxisValue :type "Float (single-precision)"))
  ;[1 1 1] 视图
  (`self.AddControllerYawInput` AxisValue))

(event `InputAxis|MovementRight`
  (params (AxisValue :type "Float (single-precision)"))
  (bind (_returnvalue_roll _returnvalue_pitch _returnvalue_yaw) (`KismetMathLibrary.BreakRotator` (`self.GetControlRotation`)))
  ;[1 1 1] WASD移动
  (`self.AddMovementInput` (`KismetMathLibrary.GetRightVector` (`KismetMathLibrary.MakeRotator` 0.0 0.0 _returnvalue_yaw)) AxisValue))

(event `InputAction|MovementJump`
  (params (Key :type "Key Structure"))
  ;[1 1 1] 跳跃
  (:`Pressed`
    (`self.Jump`))
  (:`Released`
    (`self.StopJumping`)))

(fn `UserConstructionScript`)